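; PC_Lander is the player controller for a lander game, turning player input into physics thrust on the BP_Player ship.
; BeginPlay caches the first BP_Player found in the level as PlayerShip.
; Up and Right axes apply upward and lateral forces to the ship while fuel remains, draining fuel scaled by delta time.
; Separate action inputs toggle the bottom, left and right thruster effects on press and release, independent of the fuel check.
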(event `self.ReceiveBeginPlay`
  ;[1 1 1] Gets BP_Player as PlayerShip Variable
  (bind _outactors (`GameplayStatics.GetAllActorsOfClass` "/Game/Blueprints/BP_Player.BP_Player_C"))
  (set `self.PlayerShip` (`|GetArrayItem` _outactors)))

(event `InputAxis|Up`
  (params (AxisValue :type "Float (single-precision)"))
  (bind _playership (`self.PlayerShip`))
  ;[1 1 1] Physics Thrust Up
  (if (> AxisValue 0.1)
    (`/Engine/EditorBlueprintResources/StandardMacros.IsValid` _playership
      (:`Is Valid`
        (if (> (`/Game/Blueprints/BP_Player.Fuel` _playership) 0.0)
          (`PrimitiveComponent.AddForce` (`/Game/Blueprints/BP_Player.Player` _playership) (0.0 0.0 10.0) "None" false)
          (`/Game/Blueprints/BP_Player.ChangeFuel` (`self.PlayerShip`) (* (`GameplayStatics.GetWorldDeltaSeconds`) -0.1)))))))

(event `InputAxis|Right`
  (params (AxisValue :type "Float (single-precision)"))
  (bind _playership (`self.PlayerShip`))
  ;[1 1 1] Physics Thrust Left/Right
  (if (not (`KismetMathLibrary.NearlyEqual_FloatFloat` AxisValue 0.0 0.01))
    (`/Engine/EditorBlueprintResources/StandardMacros.IsValid` _playership
      (:`Is Valid`
        (if (> (`/Game/Blueprints/BP_Player.Fuel` _playership) 0.0)
          (`PrimitiveComponent.AddForce` (`/Game/Blueprints/BP_Player.Player` _playership) (`KismetMathLibrary.MakeVector` 0.0 (* AxisValue 2.0)) "None" false)
          (`/Game/Blueprints/BP_Player.ChangeFuel` (`self.PlayerShip`) (* (`GameplayStatics.GetWorldDeltaSeconds`) -0.1)))))))

(event `InputAction|LeftThruster`
  (params (Key :type "Key Structure"))
  (bind _playership (`self.PlayerShip`))
  (bind _playership_2 (`self.PlayerShip`))
  ;[1 1 1] Activate Thrusters Niagara System
  (:`Pressed`
    (`/Engine/EditorBlueprintResources/StandardMacros.IsValid` _playership
      (:`Is Valid`
        (`/Game/Blueprints/BP_Player.ActivateThrust` _playership 1))))
  (:`Released`
    (`/Engine/EditorBlueprintResources/StandardMacros.IsValid` _playership_2
      (:`Is Valid`
        (`/Game/Blueprints/BP_Player.DeactivateThrust` _playership_2 1)))))

(event `InputAction|BottomThruster`
  (params (Key :type "Key Structure"))
  (bind _playership (`self.PlayerShip`))
  (bind _playership_2 (`self.PlayerShip`))
  ;[1 1 1] Activate Thrusters Niagara System
  (:`Pressed`
    (`/Engine/EditorBlueprintResources/StandardMacros.IsValid` _playership
      (:`Is Valid`
        (`/Game/Blueprints/BP_Player.ActivateThrust` _playership 0))))
  (:`Released`
    (`/Engine/EditorBlueprintResources/StandardMacros.IsValid` _playership_2
      (:`Is Valid`
        (`/Game/Blueprints/BP_Player.DeactivateThrust` _playership_2 0)))))

(event `InputAction|RightThruster`
  (params (Key :type "Key Structure"))
  (bind _playership (`self.PlayerShip`))
  (bind _playership_2 (`self.PlayerShip`))
  ;[1 1 1] Activate Thrusters Niagara System
  (:`Pressed`
    (`/Engine/EditorBlueprintResources/StandardMacros.IsValid` _playership_2
      (:`Is Valid`
        (`/Game/Blueprints/BP_Player.ActivateThrust` _playership_2 2))))
  (:`Released`
    (`/Engine/EditorBlueprintResources/StandardMacros.IsValid` _playership
      (:`Is Valid`
        (`/Game/Blueprints/BP_Player.DeactivateThrust` _playership 2)))))

(fn `UserConstructionScript`)