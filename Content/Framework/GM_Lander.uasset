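; GM_Lander is the game mode for a lander game, setting game-only input with a hidden cursor and handling win and lose outcomes.
; GameOverWin disables player input, shows a landing message on the HUD_Lander UI, plays sounds, then opens the NextLevel stored on the level's BP_LevelManager.
; GameOverLose shows a death message, plays an explosion sound, then reloads the current level after a delay.
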(event `self.ReceiveBeginPlay`
  (bind _returnvalue (`GameplayStatics.GetPlayerController` 0))
  ;[1 1 1] Game Mode Begin Play
  (set `PlayerController.bShowMouseCursor` false _returnvalue)
  (`WidgetBlueprintLibrary.SetInputMode_GameOnly` _returnvalue))

(event `GameOverWin`
  (bind _returnvalue (`GameplayStatics.GetPlayerController` 0))
  ;[1 1 1] Win Condition
  (`self.DisableInput` _returnvalue null)
  (bind _ashud_lander (cast `/Game/Framework/HUD_Lander` (`PlayerController.GetHUD` _returnvalue)))
  (`TextBlock.SetText` (`/Game/UI/WBP_GameLevel.TextBottomScreen` (`/Game/Framework/HUD_Lander.UI` _ashud_lander)) "You have safely landed")
  (`GameplayStatics.PlaySound2D` "/Game/Audio/Win_Sound.Win_Sound" 1.0 1.0 0.0 null null)
  (`KismetSystemLibrary.Delay` 1.0)
  (`GameplayStatics.PlaySound2D` "/Game/Audio/You_Win.You_Win" 1.0 1.0 0.0 null null)
  (`KismetSystemLibrary.Delay` 2.0)
  (bind _outactors (`GameplayStatics.GetAllActorsOfClass` "/Game/Blueprints/BP_LevelManager.BP_LevelManager_C"))
  (`GameplayStatics.OpenLevel` (`/Game/Blueprints/BP_LevelManager.NextLevel` (`|GetArrayItem` _outactors))))

(event `GameOverLose`
  ;[1 1 1] Lose Condition
  (bind _ashud_lander (cast `/Game/Framework/HUD_Lander` (`PlayerController.GetHUD` (`GameplayStatics.GetPlayerController` 0))))
  (`TextBlock.SetText` (`/Game/UI/WBP_GameLevel.TextBottomScreen` (`/Game/Framework/HUD_Lander.UI` _ashud_lander)) "You have died!")
  (`GameplayStatics.PlaySound2D` "/Game/Audio/Explosion.Explosion" 1.0 1.0 0.0 null null)
  (`KismetSystemLibrary.Delay` 4.0)
  (bind _returnvalue (`GameplayStatics.GetCurrentLevelName` true))
  (`GameplayStatics.OpenLevel` (`KismetStringLibrary.Conv_StringToName` _returnvalue)))

(fn `UserConstructionScript`)