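; BP_PlatformEnd is a landing platform for a lander game that decides whether the player wins or crashes.
; Unless flagged as the starting platform, collider overlap runs a looping timer that calls GM_Lander's GameOverWin once the player's bounds fit inside along Y.
; A platform hit at or above a speed threshold destroys the player and calls GameOverLose, even on a starting platform.
; The player is identified through BPI_Player.
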(event `self.Collider.OnComponentBeginOverlap`
  (params (OverlappedComponent :type "PrimitiveComponent Object Reference") (OtherActor :type "Actor Object Reference") (OtherComp :type "PrimitiveComponent Object Reference") (OtherBodyIndex :type Integer) (bFromSweep :type Boolean) (SweepResult :type "HitResult Structure (by ref)"))
  ;[1 1 1] Confirms Player Is In/Out Of Landing Area
  (if (and (`KismetSystemLibrary.DoesImplementInterface` OtherActor "/Game/Framework/BPI_Player.BPI_Player_C") (not (`self.IsStartingPlatform`)))
    (set `self.OverlappedActor` OtherActor)
    (bind _returnvalue (`KismetSystemLibrary.K2_SetTimer` null "IsPlayerInColliderCheck" 0.1 true))
    (set `self.CollisionCheckTimer` _returnvalue)))

(event `self.Collider.OnComponentEndOverlap`
  (params (OverlappedComponent :type "PrimitiveComponent Object Reference") (OtherActor :type "Actor Object Reference") (OtherComp :type "PrimitiveComponent Object Reference") (OtherBodyIndex :type Integer))
  ;[1 1 1] Confirms Player Is In/Out Of Landing Area
  (if (and (`KismetSystemLibrary.DoesImplementInterface` OtherActor "/Game/Framework/BPI_Player.BPI_Player_C") (not (`self.IsStartingPlatform`)))
    (`KismetSystemLibrary.K2_ClearAndInvalidateTimerHandle` (`self.CollisionCheckTimer`))))

(event `IsPlayerInColliderCheck`
  (bind (_origin _boxextent) (`KismetSystemLibrary.GetComponentBounds` (`self.Collider`)))
  (bind (_origin_2 _boxextent_2) (`self.GetActorBounds` (`self.OverlappedActor`) true false))
  ;[1 1 1] On Platform To Activate Win Condition
  (if (<= (`KismetMathLibrary.Abs` (- (.y _origin) (.y _origin_2))) (- (.y _boxextent) (.y _boxextent_2)))
    (`KismetSystemLibrary.K2_ClearAndInvalidateTimerHandle` (`self.CollisionCheckTimer`))
    (bind _asgm_lander (cast `/Game/Framework/GM_Lander` (`GameplayStatics.GetGameMode`)))
    (`/Game/Framework/GM_Lander.GameOverWin` _asgm_lander)))

(event `self.Platform.OnComponentHit`
  (params (HitComponent :type "PrimitiveComponent Object Reference") (OtherActor :type "Actor Object Reference") (OtherComp :type "PrimitiveComponent Object Reference") (NormalImpulse :type "Vector Structure") (Hit :type "HitResult Structure (by ref)"))
  ;[1 1 1] Crash And Burn To Activate Lose Condition
  (if (and (`KismetSystemLibrary.DoesImplementInterface` OtherActor "/Game/Framework/BPI_Player.BPI_Player_C") (>= (`KismetMathLibrary.VSize` (`self.GetVelocity` OtherActor)) 100.0))
    (`self.K2_DestroyActor` OtherActor)
    (bind _asgm_lander (cast `/Game/Framework/GM_Lander` (`GameplayStatics.GetGameMode`)))
    (`/Game/Framework/GM_Lander.GameOverLose` _asgm_lander)))

(fn `UserConstructionScript`)