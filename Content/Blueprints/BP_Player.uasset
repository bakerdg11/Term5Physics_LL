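; BP_Player is the player's thruster-driven craft, managing three thrusters, their sound and a fuel gauge.
; BeginPlay creates the WBP_Player widget, and ChangeFuel keeps a clamped fuel fraction in sync with its fuel bar.
; ActivateThrust and DeactivateThrust switch the centre, left or right thruster by direction, sharing one audio component.
; Deactivating any thruster stops the sound; an all-thrusters-off audio check is left unconnected.
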(event `self.ReceiveBeginPlay`
  (bind _returnvalue (`|CreateWidget` "/Game/UI/WBP_Player.WBP_Player_C"))
  (bind _output_get (set `self.UI` _returnvalue))
  (`UserWidget.AddToViewport` _output_get 0)
  (`self.ChangeFuel` 1.0))

(event `ActivateThrust`
  (params (Direction :type Integer))
  (switch `int` Direction
    (:`0`
      (if (not (`ActorComponent.IsActive` (`self.CentreThruster`)))
        (`ActorComponent.Activate` (`self.CentreThruster`) false)
        (if (not (`AudioComponent.IsPlaying` (`self.Audio`))) :!label _label
          (`AudioComponent.Play` (`self.Audio`) 0.0))))
    (:`1`
      (if (not (`ActorComponent.IsActive` (`self.LeftThruster`)))
        (`ActorComponent.Activate` (`self.LeftThruster`) false)
        (goto _label)))
    (:`2`
      (if (not (`ActorComponent.IsActive` (`self.RightThruster`)))
        (`ActorComponent.Activate` (`self.RightThruster`) false)
        (goto _label)))))

(event `DeactivateThrust`
  (params (Direction :type Integer))
  (switch `int` Direction
    (:`0`
      (if (`ActorComponent.IsActive` (`self.CentreThruster`))
        (`ActorComponent.Deactivate` (`self.CentreThruster`))
        (if (`AudioComponent.IsPlaying` (`self.Audio`)) :!label _label_2
          (`AudioComponent.Stop` (`self.Audio`)))))
    (:`1`
      (if (`ActorComponent.IsActive` (`self.LeftThruster`))
        (`ActorComponent.Deactivate` (`self.LeftThruster`))
        (goto _label_2)))
    (:`2`
      (if (`ActorComponent.IsActive` (`self.RightThruster`))
        (`ActorComponent.Deactivate` (`self.RightThruster`))
        (goto _label_2)))))

(event `ChangeFuel`
  (params (ChangeValue :type "Float (double-precision)"))
  (bind _output_get (set `self.Fuel` (`KismetMathLibrary.FClamp` (+ ChangeValue (`self.Fuel`)))))
  (`ProgressBar.SetPercent` (`/Game/UI/WBP_Player.FuelBar` (`self.UI`)) _output_get))

(event `self.ReceiveTick`
  (params (DeltaSeconds :type "Float (single-precision)")))

(fn `UserConstructionScript`)